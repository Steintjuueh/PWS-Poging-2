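; Game mode for a two-player chess game that starts the match once both players have logged in.
; When the player count reaches two after a login, it waits briefly, then assigns client-side player indices 0 and 1 to the two players.
; It then calls the chess game state to begin the multiplayer turn for player 0.
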(event `self.K2_PostLogin`
  (params (NewPlayer :type "PlayerController Object Reference"))
  (`parent.K2_PostLogin` NewPlayer)
  (bind _returnvalue (`self.GetNumPlayers`))
  (if (== _returnvalue 2)
    (`KismetSystemLibrary.Delay` 1.0)
    (`|ExecutionSequence`
      (:`then_0`
        (`self.Assign Player Indices`))
      (:`then_1`
        (`/Game/Blueprints/BP_ChessGameState.BeginPlayerTurn (multi)` (cast `/Game/Blueprints/BP_ChessGameState` (`GameplayStatics.GetGameState`) :!pure true) 0)))))

(fn `Assign Player Indices`
  (`/Game/Blueprints/BP_PlayerController.SetPlayerIndex (client)` (`self.GetPlayer` 0) 0)
  (`/Game/Blueprints/BP_PlayerController.SetPlayerIndex (client)` (`self.GetPlayer` 1) 1))

(fn `UserConstructionScript`)