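; Chess game state that tracks the active player and holds a reference to the board found at BeginPlay.
; A server event alternates turns between two players, then multicasts the new index, which fires an active-player-set dispatcher.
; A helper traces from the mouse cursor to return the hovered board tile.
; The AI hook for player 1 is empty, with its random-move logic and the delayed first-turn start left unwired.
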(event `self.ReceiveBeginPlay`
  (bind _outactors (`GameplayStatics.GetAllActorsOfClass` "/Game/Blueprints/Board/BP_Board.BP_Board_C"))
  (set `self.Board` (`|GetArrayItem` _outactors)))

(event `BeginPlayerTurn (multi)`
  (params (PlayerIndex :type Integer))
  (bind _output_get (set `self.ActivePlayerIndex` PlayerIndex))
  (`self.OnActivePlayerSet` _output_get))

(event `EndPlayerTurn (server)`
  (if (== (`self.ActivePlayerIndex`) 0)
    (set `self.ActivePlayerIndex` 1)
    (else
      (set `self.ActivePlayerIndex` 0)))
  (`self.BeginPlayerTurn (multi)` (`self.ActivePlayerIndex`))
  (if (== (`self.ActivePlayerIndex`) 1)
    (`self.Make AI Move`)))

(fn `GetActivePlayerIndex`
  (returns (ActivePlayerIndex :type Integer))
  (return (`self.ActivePlayerIndex`)))

(fn `GetBoard`
  (returns (Board :type "/Game/Blueprints/Board/BP_Board Object Reference"))
  (return (`self.Board`)))

(fn `GetHoveredTile`
  (params (PlayerController :type "PlayerController Object Reference"))
  (returns (Valid :type Boolean) (Tile :type "/Game/Blueprints/Board/Tile Structure"))
  (bind (_worldlocation _worlddirection) (`PlayerController.DeprojectMousePositionToWorld` PlayerController))
  (bind (_outhit _returnvalue) (`KismetSystemLibrary.LineTraceSingle` _worldlocation (+ _worldlocation (* _worlddirection 10000.0)) "TraceTypeQuery1"))
  (if _returnvalue
    (bind (_valid _tile) (`/Game/Blueprints/Board/BP_Board.ConvertWorldToGrid` (`self.Board`) (`.Location` (`GameplayStatics.BreakHitResult` _outhit))))
    (return _valid _tile)
    (else
      (return false))))

(fn `Make AI Move`)

(fn `UserConstructionScript`)