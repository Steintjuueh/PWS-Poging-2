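; BP_Bishop is a bishop board piece that defines which tiles it can move to from a given start tile.
; Its GetAvailableMoves calls GetTilesFromSlide for four directions, presumably the diagonals, each with a range that covers a standard chessboard.
; The results are appended into one list and returned, while the construction script just defers to the parent.
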(fn `GetAvailableMoves`
  (params (StartTile :type "/Game/Blueprints/Board/Tile Structure"))
  (returns (DestinationTiles :type "Array of /Game/Blueprints/Board/Tile Structure"))
  (locals (Output :type "Array of /Game/Blueprints/Board/Tile Structure"))
  (`|ExecutionSequence`
    (:`then_0`
      (`|ExecutionSequence`
        (:`then_0`
          (bind _crossedtiles (`self.GetTilesFromSlide` (`local.StartTile`) "NewEnumerator4" 8))
          (`KismetArrayLibrary.Array_Append` (`local.Output`) _crossedtiles))
        (:`then_1`
          (bind _crossedtiles_2 (`self.GetTilesFromSlide` (`local.StartTile`) "NewEnumerator7" 8))
          (`KismetArrayLibrary.Array_Append` (`local.Output`) _crossedtiles_2))
        (:`then_2`
          (bind _crossedtiles_3 (`self.GetTilesFromSlide` (`local.StartTile`) "NewEnumerator1" 8))
          (`KismetArrayLibrary.Array_Append` (`local.Output`) _crossedtiles_3))
        (:`then_3`
          (bind _crossedtiles_4 (`self.GetTilesFromSlide` (`local.StartTile`) "NewEnumerator5" 8))
          (`KismetArrayLibrary.Array_Append` (`local.Output`) _crossedtiles_4))))
    (:`then_1`
      (return (`local.Output`)))))

(fn `UserConstructionScript`
  (`parent.UserConstructionScript`))