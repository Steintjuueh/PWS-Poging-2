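; Chess-style pawn piece Blueprint that defines which tiles the pawn can move to.
; It overrides GetAvailableMoves, combining results from GetTilesFromSlide calls into one list.
; A forward slide reaches two tiles until the piece has moved, then one, while two single-tile angled slides use a separate capture mode for attacks.
; The event graph holds only disabled stubs, and no en passant or promotion logic appears here.
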(fn `GetAvailableMoves`
  (params (StartTile :type "/Game/Blueprints/Board/Tile Structure"))
  (returns (DestinationTiles :type "Array of /Game/Blueprints/Board/Tile Structure"))
  (locals (Output :type "Array of /Game/Blueprints/Board/Tile Structure"))
  (`|ExecutionSequence`
    (:`then_0`
      (`|ExecutionSequence`
        (:`then_0`
          ;[1 1 1] Move forward 2
          (bind _crossedtiles (`self.GetTilesFromSlide` (`local.StartTile`) "NewEnumerator0" (select `bool` (`self.GetHasEverMoved`) :`false` 2 :`true` 1) "NewEnumerator1"))
          (`KismetArrayLibrary.Array_Append` (`local.Output`) _crossedtiles))
        (:`then_1`
          ;[1 1 1] Attack (angled)
          (bind _crossedtiles_2 (`self.GetTilesFromSlide` (`local.StartTile`) "NewEnumerator4" 1 "NewEnumerator2"))
          (`KismetArrayLibrary.Array_Append` (`local.Output`) _crossedtiles_2)
          (bind _crossedtiles_3 (`self.GetTilesFromSlide` (`local.StartTile`) "NewEnumerator7" 1 "NewEnumerator2"))
          (`KismetArrayLibrary.Array_Append` (`local.Output`) _crossedtiles_3))))
    (:`then_1`
      (return (`local.Output`)))))

(fn `UserConstructionScript`
  (`parent.UserConstructionScript`))