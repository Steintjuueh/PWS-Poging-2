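; Pion is a pawn piece actor, apparently for a chess-style board game, with its behavior still unfinished.
; The construction script adds a static mesh component and zeroes the actor's rotation.
; InitialisePawn compares the Y position of a Pion found by GetActorOfClass, not necessarily itself, against BeginY, then checks FirstMove without acting on it.
; The event graph holds only disabled placeholder events.
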(fn `initialise pawn`
  (bind _returnvalue (`GameplayStatics.GetActorOfClass` "Pion_C"))
  (if (>= (.y (`self.K2_GetActorLocation` _returnvalue)) (`self.Begin y`))
    (if (`self.first move`)
      _)))

(fn `UserConstructionScript`
  (`AddComponent|NODE_AddStaticMeshComponent-0`)
  (`self.K2_SetActorRotation` (struct)))